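; House object that plays a hit sound at the impact point when the third-person character bumps its cube, debounced by a resetting DoOnce.
; If Overturnable, it drops collision and, after a delay, teleports the referenced TriggeredHouseObject to that object's NewPositionBox with its move sound.
; A Delay loop polls that sound until it ends, then restores the triggered object's hit sound and destroys this actor.
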(event OnComponentHit(Cube)
  (params (HitComponent :type Primitive%20Component%20Object%20Reference) (OtherActor :type Actor%20Object%20Reference) (OtherComp :type Primitive%20Component%20Object%20Reference) (NormalImpulse :type Vector :default "0, 0, 0") (Hit :type Hit%20Result%20Structure%20%28by%20ref%29))
  (bind _triggeredhouseobject (Variables|Default|GetTriggeredHouseObject))
  (bind _onhitaudiocomp (Variables|BP_HouseObject_C|GetOnHitAudioComp _triggeredhouseobject))
  (Utilities|Casting|CastToBP_ThirdPersonCharacter OtherActor)
  (if (not (Audio|Components|Audio|IsPlaying (Variables|Default|GetOnHitAudioComp)))
    (Utilities|FlowControl|DoOnce false :!label _label
      (:Completed
        (Utilities|FlowControl|Sequence
          (:then_0
            (Audio|PlaySoundatLocation (Variables|Default|GetHitSound) (.impactpoint Hit) "0, 0, 0" 1.0 1.0 0.0 0 0 0 0)
            (if (Variables|Default|GetOverturnable)
              (Collision|SetCollisionProfileName (Variables|Default|GetCube) "NoCollision" true :!class /Script/Engine.PrimitiveComponent)
              (Utilities|FlowControl|Delay 1.0)
              (Audio|Components|Audio|SetSound _onhitaudiocomp (Variables|BP_HouseObject_C|GetMoveSound _triggeredhouseobject))
              (Audio|Components|Audio|Play _onhitaudiocomp 0.0)
              (Transformation|SetActorTransform _triggeredhouseobject (Transformation|GetWorldTransform (Variables|BP_HouseObject_C|GetNewPositionBox _triggeredhouseobject)) false true)
              (Utilities|FlowControl|Delay 0.2 :!label _label_2)
              (if (Audio|Components|Audio|IsPlaying _onhitaudiocomp)
                (goto _label_2)
                (else
                  (Audio|Components|Audio|SetSound _onhitaudiocomp (Variables|BP_HouseObject_C|GetHitSound _triggeredhouseobject))
                  (Actor|DestroyActor)))))
          (:then_1
            (Utilities|FlowControl|Delay 1.0)
            (goto _label Reset)))))))

(event EventBeginPlay
  (Audio|Components|Audio|SetSound (Variables|Default|GetOnHitAudioComp) (Variables|Default|GetHitSound)))

(event Collision|EventActorBeginOverlap
  (params (OtherActor :type Actor%20Object%20Reference)))

(event EventTick
  (params (DeltaSeconds :type Float%20%28single-precision%29)))

(fn ConstructionScript)