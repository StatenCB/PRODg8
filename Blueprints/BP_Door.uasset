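; Two-sided door that teleports the player between two move locations, with audio cues for range and bumping.
; Each interactable area's overlap sets CanOpen and CurrentDoor on ResidenceEvilCharacter, records the active side and plays an in-range sound.
; MovePlayer disables input, waits, plays a sound, teleports to the location matching that side and restores input.
; Mesh hits from BP_ThirdPersonCharacter play a hit sound, throttled by a DoOnce with delayed reset.
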(event OnComponentBeginOverlap(InteractableArea2)
  (params (OverlappedComponent :type Primitive%20Component%20Object%20Reference) (OtherActor :type Actor%20Object%20Reference) (OtherComp :type Primitive%20Component%20Object%20Reference) (OtherBodyIndex :type Integer) (bFromSweep :type Boolean) (SweepResult :type Hit%20Result%20Structure%20%28by%20ref%29))
  (bind _asresidence_evil_character (Utilities|Casting|CastToResidenceEvilCharacter OtherActor))
  (Variables|/Script/ResidenceEvil.ResidenceEvilCharacter|SetbCanOpen _asresidence_evil_character true)
  (Variables|/Script/ResidenceEvil.ResidenceEvilCharacter|SetCurrentDoor _asresidence_evil_character self)
  (Variables|Default|SetActiveSide "Interactive Area2")
  ;[1 1 1] InRange = ljud när det går att interacta
  (Audio|Components|Audio|Play (Variables|Default|GetInRange) 0.0))

(event OnComponentBeginOverlap(InteractableArea)
  (params (OverlappedComponent :type Primitive%20Component%20Object%20Reference) (OtherActor :type Actor%20Object%20Reference) (OtherComp :type Primitive%20Component%20Object%20Reference) (OtherBodyIndex :type Integer) (bFromSweep :type Boolean) (SweepResult :type Hit%20Result%20Structure%20%28by%20ref%29))
  (bind _asresidence_evil_character (Utilities|Casting|CastToResidenceEvilCharacter OtherActor))
  (Variables|/Script/ResidenceEvil.ResidenceEvilCharacter|SetbCanOpen _asresidence_evil_character true)
  (Variables|/Script/ResidenceEvil.ResidenceEvilCharacter|SetCurrentDoor _asresidence_evil_character self)
  (Variables|Default|SetActiveSide "Interactive Area")
  (Audio|Components|Audio|Play (Variables|Default|GetInRange) 0.0))

(event OnComponentHit(MeshComponent)
  (params (HitComponent :type Primitive%20Component%20Object%20Reference) (OtherActor :type Actor%20Object%20Reference) (OtherComp :type Primitive%20Component%20Object%20Reference) (NormalImpulse :type Vector :default "0, 0, 0") (Hit :type Hit%20Result%20Structure%20%28by%20ref%29))
  (Utilities|Casting|CastToBP_ThirdPersonCharacter OtherActor)
  (if (not (Audio|Components|Audio|IsPlaying (Variables|Default|GetOnHitAudio)))
    (Utilities|FlowControl|DoOnce false :!label _label
      (:Completed
        (Utilities|FlowControl|Sequence
          (:then_0
            ;[1 1 1] HitSound = ljud när man går in i den
            (Audio|PlaySoundatLocation (Variables|Default|GetHitSound) (.location Hit) "0, 0, 0" 1.0 1.0 0.0 0 0 0 0))
          (:then_1
            (Utilities|FlowControl|Delay 1.0)
            (goto _label Reset)))))))

(event OnComponentEndOverlap(InteractableArea)
  (params (OverlappedComponent :type Primitive%20Component%20Object%20Reference) (OtherActor :type Actor%20Object%20Reference) (OtherComp :type Primitive%20Component%20Object%20Reference) (OtherBodyIndex :type Integer))
  (bind _asresidence_evil_character (Utilities|Casting|CastToResidenceEvilCharacter OtherActor))
  (Variables|/Script/ResidenceEvil.ResidenceEvilCharacter|SetbCanOpen _asresidence_evil_character false)
  (Audio|Components|Audio|Stop (Variables|Default|GetInRange)))

(event OnComponentEndOverlap(InteractableArea2)
  (params (OverlappedComponent :type Primitive%20Component%20Object%20Reference) (OtherActor :type Actor%20Object%20Reference) (OtherComp :type Primitive%20Component%20Object%20Reference) (OtherBodyIndex :type Integer))
  (bind _asresidence_evil_character (Utilities|Casting|CastToResidenceEvilCharacter OtherActor))
  (Variables|/Script/ResidenceEvil.ResidenceEvilCharacter|SetbCanOpen _asresidence_evil_character false)
  ;[1 1 1] InRange = ljud när det går att interacta
  (Audio|Components|Audio|Stop (Variables|Default|GetInRange)))

(event EventMovePlayer
  (Input|DisableInput (stale OnComponentBeginOverlap(InteractableArea) OtherActor) 0)
  ;[1 1 1] Ljud för att när man går genom dörren här, sätt delay så långt ljudet är
  (Utilities|FlowControl|Delay 2.0)
  (Audio|PlaySoundatLocation 0 (Transformation|GetActorLocation self) "0, 0, 0" 1.0 1.0 0.0 0 0 0 0)
  (if (== (Variables|Default|GetActiveSide) "Interactive Area")
    (Transformation|SetActorTransform (stale OnComponentBeginOverlap(InteractableArea) OtherActor) (Transformation|GetWorldTransform (Variables|Default|GetMoveLocation1)))
    (Input|EnableInput (stale OnComponentBeginOverlap(InteractableArea) OtherActor) 0)
    (else
      (Transformation|SetActorTransform (stale OnComponentBeginOverlap(InteractableArea2) OtherActor) (Transformation|GetWorldTransform (Variables|Default|GetMoveLocation2)))
      (Input|EnableInput (stale OnComponentBeginOverlap(InteractableArea2) OtherActor) 0))))

(fn ConstructionScript)