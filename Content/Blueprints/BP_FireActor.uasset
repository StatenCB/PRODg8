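; BP_FireActor is a flammable actor that burns with audio and spreads fire to neighbors.
; SpreadFire draws a debug capsule, plays burst and fire sounds, then after four seconds calls StartFire on overlapping BP_FireActors tagged Flammable, removing its own tag.
; Tick scales the fire audio's low-pass frequency by dot product when behind the player and prints it, though BeginPlay disables that filter.
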(event EventBeginPlay
  (Audio|Components|Audio|SetLowPassFilterEnabled (Variables|Default|GetAudioComponent) false :!class /Script/Engine.AudioComponent))

(event Collision|EventActorBeginOverlap
  (params (OtherActor :type Actor%20Object%20Reference)))

(event EventTick
  (params (DeltaSeconds :type Float%20%28single-precision%29))
  (bind _returnvalue (Game|Player|GetPlayerPawn 0))
  (bind _returnvalue_2 (Transformation|GetActorLocation))
  (bind _returnvalue_3 (Transformation|GetActorLocation _returnvalue))
  (bind _returnvalue_4 (Transformation|GetActorForwardVector _returnvalue))
  (bind _returnvalue_5 (- _returnvalue_2 _returnvalue_3))
  (bind _returnvalue_6 (Math|Vector|DotProduct _returnvalue_5 _returnvalue_4))
  (bind _returnvalue_7 (Math|Float|Absolute(Float) _returnvalue_6))
  (bind _returnvalue_8 (* _returnvalue_7 -1.7e+04))
  (bind _returnvalue_9 (+ _returnvalue_8 2e+04))
  (if (< _returnvalue_6 0.0)
    (Audio|Components|Audio|SetLowPassFilterFrequency (Variables|Default|GetAudioComponent) _returnvalue_9 :!class /Script/Engine.AudioComponent)
    (Development|PrintString (Utilities|String|ToString(Float) _returnvalue_9))))

(event EventSpreadFire
  (Rendering|Debug|DrawDebugCapsule (Transformation|GetActorLocation) 3e+01 3e+01 "0, 0, 0" "(R=1.000000,G=0.579398,B=0.063883,A=1.000000)" 1.0 3e+01)
  (Variables|Default|SetbIsSetOnFire true)
  (Audio|Components|Audio|Play (Variables|Default|GetBurstAudioComponent) 0.0)
  (Audio|Components|Audio|Play (Variables|Default|GetAudioComponent) 0.0)
  (Utilities|FlowControl|Delay 4.0)
  (for _array_element (Collision|GetOverlappingActors (Variables|Default|GetFireActorBoundsComponent) "BP_FireActor_C" :!class /Script/Engine.PrimitiveComponent)
    (if (Actor|ActorHasTag _array_element "Flammable")
      (Utilities|Array|RemoveItem (Variables|Default|GetTags self) "Flammable")
      (bind _asbp_fire_actor (Utilities|Casting|CastToBP_FireActor _array_element))
      (Class|FireActor|StartFire _asbp_fire_actor))))

(fn ConstructionScript)